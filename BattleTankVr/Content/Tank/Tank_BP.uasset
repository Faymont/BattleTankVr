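; Player tank Blueprint that binds driving, camera aiming and firing input, and passes its barrel and turret references on at BeginPlay.
; Throttle axes drive the left and right tracks separately, while aim axes rotate the azimuth gimbal and spring arm.
; A gated touch-swipe path also rotates the camera for phones once a threshold is passed.
; Fire input both calls Fire and clicks through a widget interaction component.
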(event `self.ReceiveBeginPlay`
  (`self.SetBarrelReference` (`self.Barrel`))
  (`self.SetTurretReference` (`self.Turrent`)))

(event `self.ReceiveTick`
  (params (DeltaSeconds :type "Float (single-precision)"))
  ;[0.1274 0.2086 0.4072] Touch Rotation with slides Only for Phones
)

(event `InputAction|Touch`
  (params (Key :type "Key Structure"))
  (bind (_locationx _locationy) (`PlayerController.GetInputTouchState` (`GameplayStatics.GetPlayerController` 0) "Touch1"))
  (bind _returnvalue (`KismetMathLibrary.MakeVector2D` _locationx _locationy))
  (bind (_returnvalue_x _returnvalue_y) (`KismetMathLibrary.BreakVector2D` (* (- _returnvalue (`self.PriorLoc`)) (`self.SwipeSpeed`))))
  ;[0.1274 0.2086 0.4072] Touch Rotation with slides Only for Phones
  (:`Pressed`
    (bind _output_get (set `self.StartLoc` _returnvalue))
    (set `self.PriorLoc` _output_get)
    (`/Engine/EditorBlueprintResources/StandardMacros.Gate` true :!via `Open` :!label _label
      (:`Exit`
        (if (>= (`KismetMathLibrary.VSize2D` (- _returnvalue _output_get)) (`self.SwipeThreshold`))
          (set `self.StartLoc` (100000.0 100000.0))
          (`SceneComponent.K2_AddLocalRotation` (`self.Azimuth Gimbal`) (`KismetMathLibrary.MakeRotator` 0.0 (* _returnvalue_y -1.0)) false false)
          (`SceneComponent.K2_AddLocalRotation` (`self.SpringArm`) (`KismetMathLibrary.MakeRotator` 0.0 0.0 (* _returnvalue_x -1.0)) false false)))))
  (:`Released`
    (goto _label :!via `Close`)))

(event `InputAxis|AimAzimuth`
  (params (AxisValue :type "Float (single-precision)"))
  ;[0.3146 0.5071 1] Rotation camera (If u want Gear Vr add to inputs MC Thumblestick XY)
  (`SceneComponent.K2_AddLocalRotation` (`self.Azimuth Gimbal`) (`KismetMathLibrary.MakeRotator` 0.0 0.0 AxisValue) false false))

(event `InputAction|Fire`
  (params (Key :type "Key Structure"))
  (bind _widgetinteraction (`self.WidgetInteraction`))
  ;[1 1 1] Widget interaction
  (:`Pressed`
    (`WidgetInteractionComponent.PressPointerKey` _widgetinteraction "LeftMouseButton"))
  (:`Released`
    (`WidgetInteractionComponent.ReleasePointerKey` _widgetinteraction "LeftMouseButton")))

(event `InputAxis|AimElevation`
  (params (AxisValue :type "Float (single-precision)"))
  ;[0.3146 0.5071 1] Rotation camera (If u want Gear Vr add to inputs MC Thumblestick XY)
  (`SceneComponent.K2_AddLocalRotation` (`self.SpringArm`) (`KismetMathLibrary.MakeRotator` 0.0 AxisValue) false false))

(event `InputAction|Fire`
  (params (Key :type "Key Structure"))
  (:`Pressed`
    (`self.Fire`)))

(event `InputAxis|Left Track Throttle`
  (params (AxisValue :type "Float (single-precision)"))
  (`TankTrack.SetThrottle` (`self.TankTrackL`) AxisValue))

(event `InputAxis|Right Track Throttle`
  (params (AxisValue :type "Float (single-precision)"))
  (`TankTrack.SetThrottle` (`self.TankTrackR`) AxisValue))

(fn `UserConstructionScript`)